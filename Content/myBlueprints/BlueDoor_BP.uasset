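; Blue door that the player toggles with F once the character holds the blue key.
; Box overlap caches the third-person character, enables input and opens a Gate; end overlap closes it and calls DisableInput.
; With the key, F passes the Gate into a FlipFlop that plays or reverses a Timeline lerping mesh yaw between two angles.
; Without it, a locked sound plays, then a delayed debug message names the missing key.
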(event OnComponentBeginOverlap(BlueDoor_Box)
  (params (OverlappedComponent :type Primitive%20Component%20Object%20Reference) (OtherActor :type Actor%20Object%20Reference) (OtherComp :type Primitive%20Component%20Object%20Reference) (OtherBodyIndex :type Integer) (bFromSweep :type Boolean) (SweepResult :type Hit%20Result%20Structure%20%28by%20ref%29))
  (bind _asbp_third_person_character (Utilities|Casting|CastToBP_ThirdPersonCharacter OtherActor))
  (Development|PrintString "DoorAccesed")
  (Input|EnableInput (Game|GetPlayerController 0))
  (Utilities|FlowControl|Gate true) ; enters at Open
)

(event OnComponentEndOverlap(BlueDoor_Box)
  (params (OverlappedComponent :type Primitive%20Component%20Object%20Reference) (OtherActor :type Actor%20Object%20Reference) (OtherComp :type Primitive%20Component%20Object%20Reference) (OtherBodyIndex :type Integer))
  (Utilities|Casting|CastToBP_ThirdPersonCharacter OtherActor)
  (Input|DisableInput (Game|GetPlayerController 0) 0)
  (Utilities|FlowControl|Gate true) ; enters at Close
)

(event Input|KeyboardEvents|F
  (params (Key :type Key%20Structure))
  (:Pressed
    (if (Variables|/Game/ThirdPerson/Blueprints/BP_ThirdPersonCharacter.BP_ThirdPersonCharacter_C|GethasBlueKey (stale OnComponentBeginOverlap(BlueDoor_Box) _asbp_third_person_character))
      (Utilities|FlowControl|Gate true
        (:Exit
          (Utilities|FlowControl|FlipFlop
            (:A
              (bind _door_timeline (Timeline|Timeline Play)
                (:Update
                  (Transformation|SetRelativeRotation (Variables|Default|GetStaticMesh) (Math|Rotator|MakeRotator 0.0 0.0 (Math|Float|Lerp (Variables|Default|GetOpenAngle) (Variables|Default|GetCloseAngle) _door_timeline)) false false))))
            (:B
              (Timeline|Timeline Reverse)))))
      (else
        (Audio|PlaySoundatLocation "/Game/Imports/321087__benjaminnelan__door-locked.321087__benjaminnelan__door-locked" (Transformation|GetActorLocation) "0, 0, 0" 1.0 1.0 0.0 0 0 0 0)
        (Utilities|FlowControl|Delay 0.6)
        (Development|PrintString "GetTheBlueKey")))))

(fn ConstructionScript)