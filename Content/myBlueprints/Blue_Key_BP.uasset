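; Blue key pickup that spins in the level and is collected by pressing the PICK_UP input nearby.
; Overlapping the box with BP_ThirdPersonCharacter enables input and opens a gate, while leaving closes the gate and calls DisableInput.
; A gated press sets the character's HasBlueKey flag, plays a sound, destroys the key and prints confirmation.
; Tick rotates the mesh by a fixed step, without delta-time scaling.
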(event OnComponentBeginOverlap(Box)
  (params (OverlappedComponent :type Primitive%20Component%20Object%20Reference) (OtherActor :type Actor%20Object%20Reference) (OtherComp :type Primitive%20Component%20Object%20Reference) (OtherBodyIndex :type Integer) (bFromSweep :type Boolean) (SweepResult :type Hit%20Result%20Structure%20%28by%20ref%29))
  ;[1 1 1] PICK UP THE BLUE  KEY
  (Development|PrintString "Press E to pick up")
  (bind _asbp_third_person_character (Utilities|Casting|CastToBP_ThirdPersonCharacter OtherActor))
  (Input|EnableInput (Game|GetPlayerController 0))
  (Utilities|FlowControl|Gate true) ; enters at Open
)

(event OnComponentEndOverlap(Box)
  (params (OverlappedComponent :type Primitive%20Component%20Object%20Reference) (OtherActor :type Actor%20Object%20Reference) (OtherComp :type Primitive%20Component%20Object%20Reference) (OtherBodyIndex :type Integer))
  ;[1 1 1] PICK UP THE BLUE  KEY
  (Utilities|Casting|CastToBP_ThirdPersonCharacter OtherActor)
  (Input|DisableInput (Game|GetPlayerController 0) 0)
  (Utilities|FlowControl|Gate true) ; enters at Close
)

(event EventTick
  (params (DeltaSeconds :type Float%20%28single-precision%29))
  ;[1 1 1] BASIC SPINNING
  (Transformation|AddLocalRotation (Variables|Default|GetStaticMesh) "30.000000,0.000000,0.000000" false false))

(event Input|ActionEvents|InputActionPICK_UP
  (params (Key :type Key%20Structure :default "None"))
  ;[1 1 1] PICK UP THE BLUE  KEY
  (:Pressed
    (Utilities|FlowControl|Gate true
      (:Exit
        (Variables|/Game/ThirdPerson/Blueprints/BP_ThirdPersonCharacter.BP_ThirdPersonCharacter_C|SethasBlueKey (stale OnComponentBeginOverlap(Box) _asbp_third_person_character) true)
        (Audio|PlaySoundatLocation "/Game/Imports/Key_Picked.Key_Picked" (Transformation|GetActorLocation) "0, 0, 0" 1.0 1.0 0.0 0 0 0 0)
        (Actor|DestroyActor)
        (Development|PrintString "Blue key aquired")))))

(fn ConstructionScript)